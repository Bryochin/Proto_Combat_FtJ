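; BP_Lock-On is the lock-on indicator widget, tinted yellow on BeginPlay.
; An event, noted as called by BP_Enemy on player detection, flip-flops a timer loop flag.
; A world-space update event turns the indicator toward the player camera and prints a debug string.
; The timer meant to repeat that update is unconnected, and a note says screen-space display is currently used.
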(event `self.ReceiveBeginPlay`
  (set `UserWidget.ColorAndOpacity` (struct :`R` 1.0 :`G` 0.863157 :`A` 1.0) (`self.GetWidget`)))

(event `Timer Lock-On UI`
  ; Event called in BP_Enemy when player detected. Set timer loop ON / OFF
  (`/Engine/EditorBlueprintResources/StandardMacros.FlipFlop`
    (:`A`
      (set `self.Timer Loop` true))
    (:`B`
      (set `self.Timer Loop` false))))

(event `Lock-On UI Rotation Update`
  ; Update Lock-On UI Rotation (World Space Method) [Screen Method Currently Used]
  (`KismetSystemLibrary.PrintString` "Lock-On BP !")
  (`self.K2_SetWorldRotation` (`KismetMathLibrary.FindLookAtRotation` (`self.K2_GetComponentLocation`) (`self.K2_GetComponentLocation` (`PlayerCameraManager.TransformComponent` (`GameplayStatics.GetPlayerCameraManager` 0))))))