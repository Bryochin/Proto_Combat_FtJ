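; AI controller for enemies that runs their behavior tree and exposes functions to switch their state.
; On BeginPlay it waits briefly, starts BT_Enemies and sets the E_Enemies_State Blackboard key to idle.
; SetAttackEnemiesState writes the first player's pawn as the focus target and switches the state key to attack; nothing in this controller calls it.
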(event `Set All Variables`
  ; Set Variables
)

(event `self.ReceiveBeginPlay`
  (`KismetSystemLibrary.Delay` 0.2)
  (`self.RunBehaviorTree` "/Game/Blueprints/Enemies/BT_Enemies.BT_Enemies")
  (`self.Set Idle Enemies State`))

(fn `Set Attack Enemies State`
  (bind _blackboard (`self.Blackboard`))
  (`BlackboardComponent.SetValueAsObject` _blackboard (`self.Player Focus Key Name`) (`GameplayStatics.GetPlayerPawn` 0)) ; Set the Player for BB
  (`BlackboardComponent.SetValueAsEnum` _blackboard (`self.Enemies State Key Name`) (enumliteral `/Game/Blueprints/Enemies/Enum/E_Enemies_State` "NewEnumerator1")) ; Set E_Enemies_State for BB
)

(fn `Set Idle Enemies State`
  (`BlackboardComponent.SetValueAsEnum` (`self.Blackboard`) (`self.Enemies State Key Name`) (enumliteral `/Game/Blueprints/Enemies/Enum/E_Enemies_State` "NewEnumerator3")) ; Set E_Enemies_State for BB
)

(fn `UserConstructionScript`)