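; Enemy character that supports player lock-on and reacts to kicks, weapon hits, launchers and finishers.
; Overlap shows the lock-on widget and enables Tick only until the player moves out of range; the red close-range logic is disconnected.
; Component tags select random hit animations and timelines that drive knockback or launch, with get-up after finishers and launchers.
; Also provides time-dilation hitstop, attack animation, speed/range helpers and a debug chase loop.
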(event `Auto Chase Player Debug`
  ;[1 0 0.7495] DEBUG !!!!!!!!!!!!!
  (`|AIMoveTo` self (0.0 0.0 0.0) (`GameplayStatics.GetPlayerPawn` 0) :!label _label
    (:`OnSuccess`
      _)
    (:`OnFail`
      _))
  (`KismetSystemLibrary.Delay` 2.0)
  (goto _label))

(event `Attack`
  (`KismetSystemLibrary.PrintString` (`KismetStringLibrary.Concat_StrStr` (`KismetSystemLibrary.GetGameName`) "/" "Attack"))
  (`SkeletalMeshComponent.PlayAnimation` (`self.Mesh`) (`KismetArrayLibrary.Array_Random` (`self.Random Punsh`)) false))

(event `self.ReceiveBeginPlay`
  ;[1 1 1 0.5] Just to make sure tick isn't enabled on start.
  (`SkeletalMeshComponent.PlayAnimation` (`self.Mesh`) "/Game/Frank_Pack/Frank_Fighting_Set2/Animations/Frank_FS2_Moves_Idle.Frank_FS2_Moves_Idle" true)
  (`self.SetActorTickEnabled` false))

(event `self.Lock-On Collision.OnComponentBeginOverlap`
  (params (OverlappedComponent :type "PrimitiveComponent Object Reference") (OtherActor :type "Actor Object Reference") (OtherComp :type "PrimitiveComponent Object Reference") (OtherBodyIndex :type Integer) (bFromSweep :type Boolean) (SweepResult :type "HitResult Structure (by ref)"))
  ;[0 1 0.08821 0.5] On player overlap, activates Lock-On UI + tick system to verify player's position.
  (if (`ActorComponent.ComponentHasTag` OtherComp "Player")
    (`SceneComponent.SetHiddenInGame` (`self.BP_Lock-On`) false false)
    (`/Game/Blueprints/Lock-On/BP_Lock-On.Timer Lock-On UI` (`self.BP_Lock-On`))
    (`self.SetActorTickEnabled` true)
    (`KismetSystemLibrary.PrintString` "Enabled")))

(event `self.ReceiveTick`
  (params (DeltaSeconds :type "Float (single-precision)"))
  (bind _bp_lock_on (`self.BP_Lock-On`))
  ;[0 0.4593 1 0.5] Tick Event to verify player's position and deactivate the UI and the tick when he's too far from the enemy
  (if (>= (`self.GetDistanceTo` (`GameplayStatics.GetPlayerCharacter` 0)) 800.0)
    (`/Game/ThirdPerson/Blueprints/BPI_Player.Lock-On Deactivated`) ; If Player is too far, deactivate automatically the lock-on
    (`SceneComponent.SetHiddenInGame` _bp_lock_on true false)
    (`/Game/Blueprints/Lock-On/BP_Lock-On.Timer Lock-On UI` _bp_lock_on)
    (`self.SetActorTickEnabled` false)
    (`KismetSystemLibrary.PrintString` "Disabled")))

(event `/Game/ThirdPerson/Blueprints/BPI_Player.Lock-On Activated`
  (bind _returnvalue (`WidgetComponent.GetWidget` (`self.BP_Lock-On`)))
  ;[1 0 0.04003 0.5] Change UI on Lock-On activation from the player input (input you can find in the BP_Player)
  (set `self.Is Locked-On` true)
  (set `UserWidget.ColorAndOpacity` (struct :`R` 0.152083 :`G` 0.332076 :`B` 1.0 :`A` 1.0) _returnvalue)
  (message `/Game/Blueprints/Lock-On/BPI_UI.Lock-On UI Activated` _returnvalue true))

(event `/Game/ThirdPerson/Blueprints/BPI_Player.Lock-On Deactivated`
  (bind _returnvalue (`WidgetComponent.GetWidget` (`self.BP_Lock-On`)))
  ;[1 0 0.04003 0.5] Change UI on Lock-On activation from the player input (input you can find in the BP_Player)
  (set `self.Is Locked-On` false)
  (set `UserWidget.ColorAndOpacity` (struct :`R` 1.0 :`G` 0.863157 :`A` 1.0) _returnvalue)
  (message `/Game/Blueprints/Lock-On/BPI_UI.Lock-On UI Deactivated` _returnvalue false))

(event `self.Lock-On Closed Collision.OnComponentBeginOverlap`
  (params (OverlappedComponent :type "PrimitiveComponent Object Reference") (OtherActor :type "Actor Object Reference") (OtherComp :type "PrimitiveComponent Object Reference") (OtherBodyIndex :type Integer) (bFromSweep :type Boolean) (SweepResult :type "HitResult Structure (by ref)"))
  ; Red Lock-On (When Player is Closed to Enemy to Hit Him)
)

(event `self.Lock-On Closed Collision.OnComponentEndOverlap`
  (params (OverlappedComponent :type "PrimitiveComponent Object Reference") (OtherActor :type "Actor Object Reference") (OtherComp :type "PrimitiveComponent Object Reference") (OtherBodyIndex :type Integer))
  ; Red Lock-On (When Player is Closed to Enemy to Hit Him)
)

(event `self.CapsuleComponent.OnComponentBeginOverlap`
  (params (OverlappedComponent :type "PrimitiveComponent Object Reference") (OtherActor :type "Actor Object Reference") (OtherComp :type "PrimitiveComponent Object Reference") (OtherBodyIndex :type Integer) (bFromSweep :type Boolean) (SweepResult :type "HitResult Structure (by ref)"))
  (bind (_velocity_x _velocity_y _velocity_z) (`KismetMathLibrary.BreakVector` (`MovementComponent.Velocity` (`self.CharacterMovement`))))
  (bind (_velocity_x_2 _velocity_y_2 _velocity_z_2) (`KismetMathLibrary.BreakVector` (`MovementComponent.Velocity` (`self.CharacterMovement`))))
  (bind (_velocity_x_3 _velocity_y_3 _velocity_z_3) (`KismetMathLibrary.BreakVector` (`MovementComponent.Velocity` (`self.CharacterMovement`))))
  (if (`ActorComponent.ComponentHasTag` OtherComp "Kick")
    ;[0 1 0.04588 0.5] Enemy Get Kicked
    (`SkeletalMeshComponent.PlayAnimation` (`self.Mesh`) (`KismetArrayLibrary.Array_Random` (`self.Anim Hit Kick`)) false)
    (if (`NavMovementInterface.IsFalling` (`self.CharacterMovement`))
      (bind (_direction _distancemultiplier) (`Timeline|Timeline` :!via `PlayFromStart` :!label _label)
        (:`Update`
          (bind (_returnvalue_x _returnvalue_y) (`KismetMathLibrary.BreakVector` (* (`self.GetActorForwardVector`) (* _distancemultiplier (`self.Hit Back Distance Kick`)))))
          (set `MovementComponent.Velocity` (`KismetMathLibrary.MakeVector` _returnvalue_x _returnvalue_y _velocity_z) (`self.CharacterMovement`))))
      (else
        (`self.K2_SetActorRotation` (`KismetMathLibrary.FindLookAtRotation` (`self.K2_GetActorLocation`) (`SceneComponent.K2_GetComponentLocation` (`Actor.RootComponent` (`GameplayStatics.GetPlayerCharacter` 0)))))
        (goto _label :!via `PlayFromStart`)))
    (elif (`ActorComponent.ComponentHasTag` OtherComp "Weapon")
      (if (`ActorComponent.ComponentHasTag` OtherComp "Finisher")
        ;[0.7356 0 1 0.5] Enemy Get Hit (FINISHER)
        (`SkeletalMeshComponent.PlayAnimation` (`self.Mesh`) (`KismetArrayLibrary.Array_Random` (`self.Anim Finisher Hit`)) false)
        (if (`NavMovementInterface.IsFalling` (`self.CharacterMovement`))
          (bind (_direction_2 _distancemultiplier_2) (`Timeline|Timeline Finisher` :!via `PlayFromStart` :!label _label_2)
            (:`Update`
              (bind (_returnvalue_x_2 _returnvalue_y_2) (`KismetMathLibrary.BreakVector` (* (`self.GetActorForwardVector`) (* _distancemultiplier_2 (`self.Hit Finisher Back Distance`)))))
              (set `MovementComponent.Velocity` (`KismetMathLibrary.MakeVector` _returnvalue_x_2 _returnvalue_y_2 _velocity_z_3) (`self.CharacterMovement`)))
            (:`Finished`
              (`KismetSystemLibrary.Delay` (`self.Get Up Time`))
              (`SkeletalMeshComponent.PlayAnimation` (`self.Mesh`) "/Game/Frank_Pack/Frank_Fighting_Set2/Animations/Frank_FS2_Moves_Getup_Inplace.Frank_FS2_Moves_Getup_Inplace" false)))
          (else
            (`self.K2_SetActorRotation` (`KismetMathLibrary.FindLookAtRotation` (`self.K2_GetActorLocation`) (`SceneComponent.K2_GetComponentLocation` (`Actor.RootComponent` (`GameplayStatics.GetPlayerCharacter` 0)))))
            (goto _label_2 :!via `PlayFromStart`)))
        (elif (`ActorComponent.ComponentHasTag` OtherComp "Launcher")
          ;[0 0.9612 1 0.5] Enemy Get Hit (LAUNCHER)
          (`SkeletalMeshComponent.PlayAnimation` (`self.Mesh`) (`KismetArrayLibrary.Array_Random` (`self.Anim Hit Launcher`)) false)
          (bind (_direction_3 _distancemultiplier_3) (`Timeline|Timeline Launcher` :!via `PlayFromStart`)
            (:`Update`
              (bind (_returnvalue_x_3 _returnvalue_y_3 _returnvalue_z) (`KismetMathLibrary.BreakVector` (* (`self.GetActorUpVector` (`GameplayStatics.GetPlayerPawn` 0)) (* _distancemultiplier_3 (`self.Hit Launcher Z`)))))
              (`self.LaunchCharacter` (`KismetMathLibrary.MakeVector` _returnvalue_x_3 _returnvalue_y_3 _returnvalue_z) false true))
            (:`Finished`
              (`KismetSystemLibrary.Delay` (`self.Get Up Time`))
              (`SkeletalMeshComponent.PlayAnimation` (`self.Mesh`) "/Game/Frank_Pack/Frank_Fighting_Set2/Animations/Frank_FS2_Moves_Getup_Inplace.Frank_FS2_Moves_Getup_Inplace" false)))
          (else
            ;[1 0.8807 0 0.5] Enemy Get Hit
            (`SkeletalMeshComponent.PlayAnimation` (`self.Mesh`) (`KismetArrayLibrary.Array_Random` (`self.Anim Hit`)) false)
            (bind (_direction_4 _distancemultiplier_4) (`Timeline|Timeline Hit` :!via `PlayFromStart`)
              (:`Update`
                (bind (_returnvalue_x_4 _returnvalue_y_4) (`KismetMathLibrary.BreakVector` (* (`self.GetActorForwardVector` (`GameplayStatics.GetPlayerPawn` 0)) (* _distancemultiplier_4 (`self.Hit Back Distance`)))))
                (set `MovementComponent.Velocity` (`KismetMathLibrary.MakeVector` _returnvalue_x_4 _returnvalue_y_4 _velocity_z_2) (`self.CharacterMovement`))))))))))

(fn `EndHitstop`
  (set `self.CustomTimeDilation` 1.0))

(fn `Get Ideal Range`
  (returns (`Attack Radius` :type "Float (double-precision)") (`Defend Radius` :type "Float (double-precision)"))
  (return 150.0 500.0))

(fn `Set Movement Speed`
  (params (`New Movement Speed` :type "/Game/Blueprints/Enemies/Enum/E_Enemies_Speed Enum" :default "NewEnumerator1"))
  (returns (`New Speed Value` :type "Float (double-precision)"))
  (bind _output_get (set `CharacterMovementComponent.MaxWalkSpeed` (select `/Game/Blueprints/Enemies/Enum/E_Enemies_Speed` `New Movement Speed` :`NewEnumerator0` 200.0 :`NewEnumerator2` 400.0 :!type "Float (single-precision)") (`self.CharacterMovement`)))
  (return _output_get))

(fn `SetMovementSpeed`
  (params (`New Movement Speed` :type "/Game/Blueprints/Enemies/Enum/E_Enemies_Speed Enum" :default "NewEnumerator1")))

(fn `StartHitstop`
  (params (Duration :type "Float (double-precision)"))
  (set `self.CustomTimeDilation` 0.0)
  (`KismetSystemLibrary.K2_SetTimer` null "EndHitstop" Duration))

(fn `Sword Hitbox Activation`
  (returns (`Box Collision` :type "Array of BoxComponent Object Reference"))
  (return))

(fn `UserConstructionScript`)